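; Trap actor that damages the player character when it walks into the trigger box.
; On overlap it casts to BP_CustomTPS, calls its damaged event, and spawns an enlarged campfire particle effect above itself.
; It then removes its box and mesh at once, and after a short delay destroys the effect and the actor, making it single-use.
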(event `self.Box.OnComponentBeginOverlap`
  (params (OverlappedComponent :type "PrimitiveComponent Object Reference") (OtherActor :type "Actor Object Reference") (OtherComp :type "PrimitiveComponent Object Reference") (OtherBodyIndex :type Integer) (bFromSweep :type Boolean) (SweepResult :type "HitResult Structure (by ref)"))
  (bind _returnvalue_location (`KismetMathLibrary.BreakTransform` (`self.GetTransform`)))
  (bind _asbp_custom_tps (cast `/Game/Blueprints/BP_CustomTPS` OtherActor))
  (`/Game/Blueprints/BP_CustomTPS.Damaged` _asbp_custom_tps)
  (bind _returnvalue (`GameplayStatics.SpawnEmitterAtLocation` "/Game/Assets/Dreamscape/Effects/P_Stylized_Campfire.P_Stylized_Campfire" (+ _returnvalue_location (0.0 0.0 50.0)) (struct) (3.0 3.0 3.0) false))
  (`ActorComponent.K2_DestroyComponent` (`self.Box`))
  (`ActorComponent.K2_DestroyComponent` (`self.StaticMesh`))
  (`KismetSystemLibrary.Delay` 1.0)
  (`ActorComponent.K2_DestroyComponent` _returnvalue)
  (`self.K2_DestroyActor`))

(fn `UserConstructionScript`)